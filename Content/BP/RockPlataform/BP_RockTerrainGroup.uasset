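; BP_RockTerrainGroup is a rock terrain group of eight static mesh components, varied procedurally for level dressing.
; The Construction Script gives each mesh a random non-uniform scale, stretched more horizontally than vertically, and a random local offset multiplied by EscalaOffset.
; The randomness is unseeded, so the layout can change whenever construction reruns; the event graph has no active logic.
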(event EventBeginPlay)

(event Collision|EventActorBeginOverlap
  (params (OtherActor :type Actor%20Object%20Reference)))

(event EventTick
  (params (DeltaSeconds :type Float%20%28single-precision%29)))

(fn ConstructionScript
  (for _array_element (Utilities|Array|MakeArray (Variables|Default|GetStaticMesh6) (Variables|Default|GetStaticMesh5) (Variables|Default|GetStaticMesh4) (Variables|Default|GetStaticMesh) (Variables|Default|GetStaticMesh1) (Variables|Default|GetStaticMesh2) (Variables|Default|GetStaticMesh3) (Variables|Default|GetStaticMesh7))
    (Transformation|SetRelativeScale3D _array_element (Math|Vector|MakeVector (Math|Random|RandomFloatinRange 1.0 2.0) (Math|Random|RandomFloatinRange 1.0 2.0) (Math|Random|RandomFloatinRange 1.0 1.2)))
    (Transformation|AddLocalOffset _array_element (* (Math|Vector|MakeVector (Math|Random|RandomFloatinRange -1e+01 1e+01) (Math|Random|RandomFloatinRange -1e+01 1e+01) (Math|Random|RandomFloatinRange -1e+01 1e+01)) (Variables|Default|GetEscalaOffset)) false false)))