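; Trigger volume that starts a dialogue automatically when BP_Pato walks into it, then destroys itself when the duck leaves.
; On BeginPlay, if LlaveKey is absent from the game instance's key list, it loads the NoTieneKey row and key-granting settings into BPDialogueComp.
; On overlap it registers as the duck's DialogueActor and, after a short delay, forces the interaction via InteractuarAlasMalas.
; The SiTieneKey row assignment is unwired.
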(event OnComponentBeginOverlap(Box)
  (params (OverlappedComponent :type Primitive%20Component%20Object%20Reference) (OtherActor :type Actor%20Object%20Reference) (OtherComp :type Primitive%20Component%20Object%20Reference) (OtherBodyIndex :type Integer) (bFromSweep :type Boolean) (SweepResult :type Hit%20Result%20Structure%20%28by%20ref%29))
  (bind _asbp_pato (Utilities|Casting|CastToBP_Pato OtherActor))
  (Variables|/Game/BP/BP_Pato.BP_Pato_C|SetDialogueActor _asbp_pato self)
  (Utilities|FlowControl|Delay 0.2)
  (Variables|/Game/BP/BP_Pato.BP_Pato_C|SetbInteractuable _asbp_pato true)
  (Default|InteractuarAlasMalas _asbp_pato))

(event OnComponentEndOverlap(Box)
  (params (OverlappedComponent :type Primitive%20Component%20Object%20Reference) (OtherActor :type Actor%20Object%20Reference) (OtherComp :type Primitive%20Component%20Object%20Reference) (OtherBodyIndex :type Integer))
  (Utilities|Casting|CastToBP_Pato OtherActor)
  (Variables|/Game/BP/BP_Pato.BP_Pato_C|SetbInteractuable (stale OnComponentBeginOverlap(Box) _asbp_pato) false)
  (Actor|DestroyActor))

(event EventBeginPlay
  (bind _bp_dialoguecomp (Variables|Default|GetBP_DialogueComp))
  (bind _no_tiene_key (Variables|Default|Getno%20tiene%20key))
  (bind _asbp_game_instance (Utilities|Casting|CastToBP_GameInstance (Game|GetGameInstance)))
  (if (== (Utilities|Array|FindItem (Variables|/Game/BP/SaveGame/BP_GameInstance.BP_GameInstance_C|GetListaKeys _asbp_game_instance) (Variables|Default|GetLlave%28Key%29?)) -1)
    (Variables|/Game/BP/Dialogo/BP_DialogueComp.BP_DialogueComp_C|SetRow%20Name_0 _bp_dialoguecomp _no_tiene_key)
    (Variables|/Game/BP/Dialogo/BP_DialogueComp.BP_DialogueComp_C|SetRow%20Name _bp_dialoguecomp _no_tiene_key)
    (Variables|/Game/BP/Dialogo/BP_DialogueComp.BP_DialogueComp_C|SetDarLlave _bp_dialoguecomp (Variables|Default|GetDar%20Llave))
    (Variables|/Game/BP/Dialogo/BP_DialogueComp.BP_DialogueComp_C|SetItem%20key _bp_dialoguecomp (Variables|Default|GetItem%20Key))))

(fn ConstructionScript)