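; BP_ZonaMuerta is a dead-zone trigger that returns the BP_Pato player to a Target actor's location when it overlaps the Box.
; On overlap it disables input and shows a WBP_FadeLevels fade-in widget for a short delay.
; It then teleports the pato to the Target, swaps in a fade-out instance of the same widget and re-enables input.
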(event OnComponentBeginOverlap(Box)
  (params (OverlappedComponent :type Primitive%20Component%20Object%20Reference) (OtherActor :type Actor%20Object%20Reference) (OtherComp :type Primitive%20Component%20Object%20Reference) (OtherBodyIndex :type Integer) (bFromSweep :type Boolean) (SweepResult :type Hit%20Result%20Structure%20%28by%20ref%29))
  (bind _returnvalue (Game|GetPlayerController 0))
  (bind _returnvalue_2 (Game|GetPlayerController 0))
  (bind _asbp_pato (Utilities|Casting|CastToBP_Pato OtherActor))
  (Input|DisableInput _asbp_pato _returnvalue_2)
  (bind _returnvalue_3 (UserInterface|CreateWidget "/Game/Widget/WBP_FadeLevels.WBP_FadeLevels_C" _returnvalue_2))
  (UserInterface|Viewport|AddtoViewport _returnvalue_3 0)
  (Utilities|FlowControl|Delay 1.0)
  (Transformation|SetActorLocation _asbp_pato (Transformation|GetActorLocation (Variables|Default|GetTarget)) false true)
  (Widget|RemovefromParent _returnvalue_3)
  (bind _returnvalue_4 (UserInterface|CreateWidget "/Game/Widget/WBP_FadeLevels.WBP_FadeLevels_C" _returnvalue false))
  (UserInterface|Viewport|AddtoViewport _returnvalue_4 0)
  (Input|EnableInput _asbp_pato _returnvalue))

(fn ConstructionScript)