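; BP_TextFlotante is a floating text Blueprint that shows localized text through its Widget component.
; On BeginPlay it loads the BP_SaveGame slot to read the language setting and looks up RowName in the CSV_PatodaLaVida data table.
; It picks the Spanish, English, Portuguese or French column and passes that text, with configurable color and font, to a new WBP_TextAlong widget.
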(event EventBeginPlay
  (bind _returnvalue (SaveGame|LoadGamefromSlot "a"))
  (bind _asbp_save_game (Utilities|Casting|CastToBP_SaveGame _returnvalue))
  (Variables|Default|SetAs%20BP%20Save%20Game _asbp_save_game)
  (bind _returnvalue_2 (Utilities|GetDataTableRow "/Game/DataTable/CSV_PatodaLaVida_DataTable.CSV_PatodaLaVida_DataTable" (Variables|Default|GetRow%20Name))
    (:then
      (bind _returnvalue_3 (UserInterface|CreateWidget "/Game/Widget/WBP_TextAlong.WBP_TextAlong_C" (Game|GetPlayerController 0) (Variables|Default|GetIn%20Color%20And%20Opacity) (Variables|Default|GetIn%20Font%20Info) (Utilities|Text|ToText(String) (Utilities|Select :Index (.lenguaje (Variables|/Game/BP/SaveGame/BP_SaveGame.BP_SaveGame_C|GetVar%20Ajustes%20Juego (Variables|Default|GetAs%20BP%20Save%20Game))) :Option%200 (.Español (Utilities|Struct|BreakLenguajeStructure _returnvalue_2)) :Option%201 (.Ingles (Utilities|Struct|BreakLenguajeStructure _returnvalue_2)) :Option%202 (.Portugues (Utilities|Struct|BreakLenguajeStructure _returnvalue_2)) :Option%203 (.Frances (Utilities|Struct|BreakLenguajeStructure _returnvalue_2))))))
      (UserInterface|SetWidget (Variables|Default|GetWidget) _returnvalue_3))))

(fn ConstructionScript)