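; Dialogue component that shows localized, multi-line conversations in a WBP_Dialogo widget each time the player interacts.
; Each DataTable row supplies speaker, text, next row and table, and an end flag, forming a linked chain starting at RowName0.
; The save game loaded on BeginPlay selects among Spanish, English, Portuguese and French text.
; Ending removes the widget, restores game-only input and calls SwitchDistanceCamera(false) on the player.
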(event Custom|End%20Dialogo
  (Utilities|IsValid (Variables|Default|GetWB%20Dialogo)
    (:Is%20Valid
      (Widget|RemovefromParent (Variables|Default|GetWB%20Dialogo))
      (Variables|Default|SetEnd%20Dialogo? false)
      (Variables|Default|SetWB%20Dialogo 0)
      (Input|SetInputModeGameOnly (Game|GetPlayerController 0) false)
      (Default|SwitchDistanceCamera (stale EventDiagInteraciton PlayerRef) false))))

(event EventBeginPlay
  (bind _returnvalue (SaveGame|LoadGamefromSlot "a"))
  (bind _asbp_save_game (Utilities|Casting|CastToBP_SaveGame _returnvalue))
  (Variables|Default|SetAs%20BP%20Save%20Game _asbp_save_game))

(event EventDiagInteraciton
  (params (PlayerRef :type BP%20Pato%20Object%20Reference))
  (if (Variables|Default|GetEnd%20Dialogo?)
    (Widget|RemovefromParent (Variables|Default|GetWB%20Dialogo))
    (Variables|Default|SetEnd%20Dialogo? false)
    (Variables|Default|SetWB%20Dialogo 0)
    (Input|SetInputModeGameOnly (Game|GetPlayerController 0) false)
    (Default|SwitchDistanceCamera PlayerRef false)
    (else
      (Utilities|IsValid (Variables|Default|GetWB%20Dialogo)
        (:Is%20Valid
          (bind _returnvalue (Utilities|GetDataTableRow (Variables|Default|GetData%20Table) (Variables|Default|GetRow%20Name))
            (:then
              (Variables|/Game/Widget/WBP_Dialogo.WBP_Dialogo_C|SetDiagParrafoText (Variables|Default|GetWB%20Dialogo) (Utilities|Text|ToText(String) (Utilities|Select :Index (.Lenguaje (Utilities|Struct|BreakAjustesJuego (Variables|/Game/BP/SaveGame/BP_SaveGame.BP_SaveGame_C|GetVar%20Ajustes%20Juego (Variables|Default|GetAs%20BP%20Save%20Game)))) :Option%200 (.Español (Utilities|Struct|BreakDialogoStruct _returnvalue)) :Option%201 (.Ingles (Utilities|Struct|BreakDialogoStruct _returnvalue)) :Option%202 (.Portugues (Utilities|Struct|BreakDialogoStruct _returnvalue)) :Option%203 (.Frances (Utilities|Struct|BreakDialogoStruct _returnvalue)))))
              (Variables|Default|SetRow%20Name (.Row (Utilities|Struct|BreakDialogoStruct _returnvalue)))
              (Variables|Default|SetData%20Table (.DataTable (Utilities|Struct|BreakDialogoStruct _returnvalue)))
              (Variables|Default|SetEnd%20Dialogo? (.EndDialogo? (Utilities|Struct|BreakDialogoStruct _returnvalue)))
              (Variables|/Game/Widget/WBP_Dialogo.WBP_Dialogo_C|SetDiagNombreText (Variables|Default|GetWB%20Dialogo) (Utilities|Text|ToText(String) (.Nombre (Utilities|Struct|BreakDialogoStruct _returnvalue)))))))
        (:Is%20Not%20Valid
          (Variables|Default|SetRow%20Name (Variables|Default|GetRow%20Name_0))
          (bind _returnvalue_2 (Utilities|GetDataTableRow (Variables|Default|GetData%20Table) (Variables|Default|GetRow%20Name))
            (:then
              (bind _returnvalue_3 (UserInterface|CreateWidget "/Game/Widget/WBP_Dialogo.WBP_Dialogo_C" (Game|GetPlayerController 0) (Utilities|Text|ToText(String) (.Nombre (Utilities|Struct|BreakDialogoStruct _returnvalue_2))) (Utilities|Text|ToText(String) (Utilities|Select :Index (.Lenguaje (Utilities|Struct|BreakAjustesJuego (Variables|/Game/BP/SaveGame/BP_SaveGame.BP_SaveGame_C|GetVar%20Ajustes%20Juego (Variables|Default|GetAs%20BP%20Save%20Game)))) :Option%200 (.Español (Utilities|Struct|BreakDialogoStruct _returnvalue_2)) :Option%201 (.Ingles (Utilities|Struct|BreakDialogoStruct _returnvalue_2)) :Option%202 (.Portugues (Utilities|Struct|BreakDialogoStruct _returnvalue_2)) :Option%203 (.Frances (Utilities|Struct|BreakDialogoStruct _returnvalue_2))))))
              (Variables|Default|SetRow%20Name (.Row (Utilities|Struct|BreakDialogoStruct _returnvalue_2)))
              (Variables|Default|SetData%20Table (.DataTable (Utilities|Struct|BreakDialogoStruct _returnvalue_2)))
              (Variables|Default|SetEnd%20Dialogo? (.EndDialogo? (Utilities|Struct|BreakDialogoStruct _returnvalue_2)))
              (bind _output_get (Variables|Default|SetWB%20Dialogo _returnvalue_3))
              (UserInterface|Viewport|AddtoViewport _output_get 0)
              (Input|SetInputModeGameandUI (Game|GetPlayerController 0) _output_get "DoNotLock" true false))))))))