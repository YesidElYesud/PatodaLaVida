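; Level-change trigger that shows a prompt while the duck (BP_Pato) is inside its box and loads another level on a quack event.
; BeginPlay builds a hidden WBP_TextAlongIdioma widget with keyboard and Xbox text, toggled by box overlaps.
; HizoQuack, fired from outside this graph, adds a fade widget, waits briefly, then opens LevelName.
; The construction script applies the configurable box extent and widget position.
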(event OnComponentBeginOverlap(Box)
  (params (OverlappedComponent :type Primitive%20Component%20Object%20Reference) (OtherActor :type Actor%20Object%20Reference) (OtherComp :type Primitive%20Component%20Object%20Reference) (OtherBodyIndex :type Integer) (bFromSweep :type Boolean) (SweepResult :type Hit%20Result%20Structure%20%28by%20ref%29))
  (Utilities|Casting|CastToBP_Pato OtherActor)
  (Rendering|SetVisibility (Variables|Default|GetWidget) true false))

(event OnComponentEndOverlap(Box)
  (params (OverlappedComponent :type Primitive%20Component%20Object%20Reference) (OtherActor :type Actor%20Object%20Reference) (OtherComp :type Primitive%20Component%20Object%20Reference) (OtherBodyIndex :type Integer))
  (Utilities|Casting|CastToBP_Pato OtherActor)
  (Rendering|SetVisibility (Variables|Default|GetWidget) false false))

(event EventBeginPlay
  (bind _returnvalue (UserInterface|CreateWidget "/Game/Widget/WBP_TextAlongIdioma.WBP_TextAlongIdioma_C" (Game|GetPlayerController 0) (Variables|Default|GetIn%20Color%20And%20Opacity) (Variables|Default|GetIn%20Font%20Info) (Variables|Default|GetXbox) (Variables|Default|GetKeyBoard)))
  (UserInterface|SetWidget (Variables|Default|GetWidget) _returnvalue)
  (Rendering|SetVisibility (Variables|Default|GetWidget) false false))

(event EventHizoQuack
  (bind _returnvalue (UserInterface|CreateWidget "/Game/Widget/WBP_FadeLevels.WBP_FadeLevels_C" (Game|GetPlayerController 0)))
  (UserInterface|Viewport|AddtoViewport _returnvalue 0)
  (Utilities|FlowControl|Delay 1.0)
  (Game|OpenLevel(byName) (Variables|Default|GetLevel%20Name)))

(fn ConstructionScript
  (Components|Box|SetBoxExtent (Variables|Default|GetBox) (Variables|Default|GetIn%20Box%20Extent) true)
  (Transformation|SetRelativeLocation (Variables|Default|GetWidget) (Variables|Default|GetWidget%20Location) false false))