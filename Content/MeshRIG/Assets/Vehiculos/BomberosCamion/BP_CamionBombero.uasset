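; BP_CamionBombero is a fire truck hazard with a sweeping part that pushes the duck character BP_Pato.
; A timeline started on BeginPlay drives the yaw of a Scene component across an arc of up to 170 degrees.
; While BP_Pato overlaps the Capsule, a second timeline relaunches it every update along the Arrow's forward vector, overriding horizontal velocity, and stops on end overlap.
; Debug prints remain.
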(event OnComponentBeginOverlap(Capsule)
  (params (OverlappedComponent :type Primitive%20Component%20Object%20Reference) (OtherActor :type Actor%20Object%20Reference) (OtherComp :type Primitive%20Component%20Object%20Reference) (OtherBodyIndex :type Integer) (bFromSweep :type Boolean) (SweepResult :type Hit%20Result%20Structure%20%28by%20ref%29))
  (bind _asbp_pato (Utilities|Casting|CastToBP_Pato OtherActor))
  (Timeline|Timeline_0 Play
    (:Update
      (Character|LaunchCharacter _asbp_pato (* (Math|Vector|GetForwardVector (Variables|Default|GetArrow)) 1400) true false)
      (Development|PrintString "Hello"))))

(event OnComponentEndOverlap(Capsule)
  (params (OverlappedComponent :type Primitive%20Component%20Object%20Reference) (OtherActor :type Actor%20Object%20Reference) (OtherComp :type Primitive%20Component%20Object%20Reference) (OtherBodyIndex :type Integer))
  (Utilities|Casting|CastToBP_Pato OtherActor)
  (Timeline|Timeline_0 Stop
    (:Update
      (Character|LaunchCharacter (stale OnComponentBeginOverlap(Capsule) _asbp_pato) (* (Math|Vector|GetForwardVector (Variables|Default|GetArrow)) 1400) true false)
      (Development|PrintString "Hello"))))

(event EventBeginPlay
  (bind _newtrack_0 (Timeline|Timeline Play)
    (:Update
      (Transformation|SetRelativeRotation (Variables|Default|GetScene) (Math|Rotator|MakeRotator 0.0 0.0 (Math|Float|MapRangeClamped _newtrack_0 0.0 1.0 0.0 1.7e+02)) false false))))

(fn ConstructionScript)